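; BP_Origin is a wheeled robot assembly target where printed parts and electronics are installed by overlapping slot colliders.
; Each slot casts the overlapping actor to BP_PrintedParts or BP_Electronics and checks its Spec or CompNumber.
; A match, accepted once per slot, destroys the part and reveals the pre-placed mesh.
; A wrong index increments ErrorCount and prints a Russian error message; the ErrorCounter function is a stub returning zero.
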(event OnComponentBeginOverlap(BC_LeftWheel)
  (params (OverlappedComponent :type Primitive%20Component%20Object%20Reference) (OtherActor :type Actor%20Object%20Reference) (OtherComp :type Primitive%20Component%20Object%20Reference) (OtherBodyIndex :type Integer) (bFromSweep :type Boolean) (SweepResult :type Hit%20Result%20Structure%20%28by%20ref%29))
  (bind _asbp_printed_parts (Utilities|Casting|CastToBP_PrintedParts OtherActor))
  (if (== (Variables|/Game/MyLogic/BP_PrintedParts.BP_PrintedParts_C|GetSpec _asbp_printed_parts) 0)
    (Utilities|FlowControl|DoOnce false
      (:Completed
        (Actor|DestroyActor _asbp_printed_parts)
        (Rendering|SetVisibility (Variables|Default|GetSM_LeftWheel) true false)))
    (else
      (bind _output_get (Variables|Default|SetErrorCount (+ (Variables|Default|GetErrorCount) 1)))
      (Development|PrintString (Utilities|String|Append "Текущее количество ошибок: " (Utilities|String|ToString(Integer) _output_get) ". Нееверная установка компонента.")))))

(event OnComponentBeginOverlap(BC_RightWheel)
  (params (OverlappedComponent :type Primitive%20Component%20Object%20Reference) (OtherActor :type Actor%20Object%20Reference) (OtherComp :type Primitive%20Component%20Object%20Reference) (OtherBodyIndex :type Integer) (bFromSweep :type Boolean) (SweepResult :type Hit%20Result%20Structure%20%28by%20ref%29))
  (bind _asbp_printed_parts (Utilities|Casting|CastToBP_PrintedParts OtherActor))
  (if (== (Variables|/Game/MyLogic/BP_PrintedParts.BP_PrintedParts_C|GetSpec _asbp_printed_parts) 0)
    (Utilities|FlowControl|DoOnce false
      (:Completed
        (Actor|DestroyActor _asbp_printed_parts)
        (Rendering|SetVisibility (Variables|Default|GetSM_RightWheel) true false)))
    (else
      (bind _output_get (Variables|Default|SetErrorCount (+ (Variables|Default|GetErrorCount) 1)))
      (Development|PrintString (Utilities|String|Append "Текущее количество ошибок: " (Utilities|String|ToString(Integer) _output_get) ". Нееверная установка компонента.")))))

(event OnComponentBeginOverlap(BC_RightMountWheel)
  (params (OverlappedComponent :type Primitive%20Component%20Object%20Reference) (OtherActor :type Actor%20Object%20Reference) (OtherComp :type Primitive%20Component%20Object%20Reference) (OtherBodyIndex :type Integer) (bFromSweep :type Boolean) (SweepResult :type Hit%20Result%20Structure%20%28by%20ref%29))
  (bind _asbp_printed_parts (Utilities|Casting|CastToBP_PrintedParts OtherActor))
  (if (== (Variables|/Game/MyLogic/BP_PrintedParts.BP_PrintedParts_C|GetSpec _asbp_printed_parts) 1)
    (Utilities|FlowControl|DoOnce false
      (:Completed
        (Actor|DestroyActor _asbp_printed_parts)
        (Rendering|SetVisibility (Variables|Default|GetSM_RightMountWheel) true false)))
    (else
      (bind _output_get (Variables|Default|SetErrorCount (+ (Variables|Default|GetErrorCount) 1)))
      (Development|PrintString (Utilities|String|Append "Текущее количество ошибок:" (Utilities|String|ToString(Integer) _output_get) ". Нееверная установка компонента.")))))

(event OnComponentBeginOverlap(BC_LeftMountWheel)
  (params (OverlappedComponent :type Primitive%20Component%20Object%20Reference) (OtherActor :type Actor%20Object%20Reference) (OtherComp :type Primitive%20Component%20Object%20Reference) (OtherBodyIndex :type Integer) (bFromSweep :type Boolean) (SweepResult :type Hit%20Result%20Structure%20%28by%20ref%29))
  (bind _asbp_printed_parts (Utilities|Casting|CastToBP_PrintedParts OtherActor))
  (if (== (Variables|/Game/MyLogic/BP_PrintedParts.BP_PrintedParts_C|GetSpec _asbp_printed_parts) 1)
    (Utilities|FlowControl|DoOnce false
      (:Completed
        (Actor|DestroyActor _asbp_printed_parts)
        (Rendering|SetVisibility (Variables|Default|GetSM_LeftMountWheel) true false)))
    (else
      (bind _output_get (Variables|Default|SetErrorCount (+ (Variables|Default|GetErrorCount) 1)))
      (Development|PrintString (Utilities|String|Append "Текущее количество ошибок:" (Utilities|String|ToString(Integer) _output_get) ". Нееверная установка компонента.")))))

(event OnComponentBeginOverlap(BC_CasterWheel)
  (params (OverlappedComponent :type Primitive%20Component%20Object%20Reference) (OtherActor :type Actor%20Object%20Reference) (OtherComp :type Primitive%20Component%20Object%20Reference) (OtherBodyIndex :type Integer) (bFromSweep :type Boolean) (SweepResult :type Hit%20Result%20Structure%20%28by%20ref%29))
  (bind _asbp_printed_parts (Utilities|Casting|CastToBP_PrintedParts OtherActor))
  (if (== (Variables|/Game/MyLogic/BP_PrintedParts.BP_PrintedParts_C|GetSpec _asbp_printed_parts) 2)
    (Utilities|FlowControl|DoOnce false
      (:Completed
        (Actor|DestroyActor _asbp_printed_parts)
        (Rendering|SetVisibility (Variables|Default|GetSM_CasterWheel) true false)))
    (else
      (bind _output_get (Variables|Default|SetErrorCount (+ (Variables|Default|GetErrorCount) 1)))
      (Development|PrintString (Utilities|String|Append "Текущее количество ошибок:" (Utilities|String|ToString(Integer) _output_get) ". Нееверная установка компонента.")))))

(event OnComponentBeginOverlap(BC_LeftMotor)
  (params (OverlappedComponent :type Primitive%20Component%20Object%20Reference) (OtherActor :type Actor%20Object%20Reference) (OtherComp :type Primitive%20Component%20Object%20Reference) (OtherBodyIndex :type Integer) (bFromSweep :type Boolean) (SweepResult :type Hit%20Result%20Structure%20%28by%20ref%29))
  (bind _asbp_electronics (Utilities|Casting|CastToBP_Electronics OtherActor))
  (if (== (Variables|/Game/MyLogic/BP_Electronics.BP_Electronics_C|GetCompNumber _asbp_electronics) 0)
    (Utilities|FlowControl|DoOnce false
      (:Completed
        (Actor|DestroyActor _asbp_electronics)
        (Rendering|SetVisibility (Variables|Default|GetSM_LeftMotor) true false)))
    (else
      (bind _output_get (Variables|Default|SetErrorCount (+ (Variables|Default|GetErrorCount) 1)))
      (Development|PrintString (Utilities|String|Append "Текущее количество ошибок" (Utilities|String|ToString(Integer) _output_get) ". Нееверная установка компонента")))))

(event OnComponentBeginOverlap(BC_RightMotor)
  (params (OverlappedComponent :type Primitive%20Component%20Object%20Reference) (OtherActor :type Actor%20Object%20Reference) (OtherComp :type Primitive%20Component%20Object%20Reference) (OtherBodyIndex :type Integer) (bFromSweep :type Boolean) (SweepResult :type Hit%20Result%20Structure%20%28by%20ref%29))
  (bind _asbp_electronics (Utilities|Casting|CastToBP_Electronics OtherActor))
  (if (== (Variables|/Game/MyLogic/BP_Electronics.BP_Electronics_C|GetCompNumber _asbp_electronics) 0)
    (Utilities|FlowControl|DoOnce false
      (:Completed
        (Actor|DestroyActor _asbp_electronics)
        (Rendering|SetVisibility (Variables|Default|GetSM_RightMotor) true false)))
    (else
      (bind _output_get (Variables|Default|SetErrorCount (+ (Variables|Default|GetErrorCount) 1)))
      (Development|PrintString (Utilities|String|Append "Текущее количество ошибок" (Utilities|String|ToString(Integer) _output_get) ". Нееверная установка компонента")))))

(event OnComponentBeginOverlap(BC_Driver)
  (params (OverlappedComponent :type Primitive%20Component%20Object%20Reference) (OtherActor :type Actor%20Object%20Reference) (OtherComp :type Primitive%20Component%20Object%20Reference) (OtherBodyIndex :type Integer) (bFromSweep :type Boolean) (SweepResult :type Hit%20Result%20Structure%20%28by%20ref%29))
  (bind _asbp_electronics (Utilities|Casting|CastToBP_Electronics OtherActor))
  (if (== (Variables|/Game/MyLogic/BP_Electronics.BP_Electronics_C|GetCompNumber _asbp_electronics) 1)
    (Utilities|FlowControl|DoOnce false
      (:Completed
        (Actor|DestroyActor _asbp_electronics)
        (Rendering|SetVisibility (Variables|Default|GetSM_Driver) true false)))
    (else
      (bind _output_get (Variables|Default|SetErrorCount (+ (Variables|Default|GetErrorCount) 1)))
      (Development|PrintString (Utilities|String|Append "Текущее количество ошибок" (Utilities|String|ToString(Integer) _output_get) ". Нееверная установка компонента"))
      (CallFunction|ErrorCounter _output_get))))

(event OnComponentBeginOverlap(BC_Pico)
  (params (OverlappedComponent :type Primitive%20Component%20Object%20Reference) (OtherActor :type Actor%20Object%20Reference) (OtherComp :type Primitive%20Component%20Object%20Reference) (OtherBodyIndex :type Integer) (bFromSweep :type Boolean) (SweepResult :type Hit%20Result%20Structure%20%28by%20ref%29))
  (bind _asbp_electronics (Utilities|Casting|CastToBP_Electronics OtherActor))
  (if (== (Variables|/Game/MyLogic/BP_Electronics.BP_Electronics_C|GetCompNumber _asbp_electronics) 2)
    (Utilities|FlowControl|DoOnce false
      (:Completed
        (Actor|DestroyActor _asbp_electronics)
        (Rendering|SetVisibility (Variables|Default|GetSM_Pico) true false)))
    (else
      (bind _output_get (Variables|Default|SetErrorCount (+ (Variables|Default|GetErrorCount) 1)))
      (Development|PrintString (Utilities|String|Append "Текущее количество ошибок" (Utilities|String|ToString(Integer) _output_get) ". Нееверная установка компонента"))
      (CallFunction|ErrorCounter _output_get))))

(event OnComponentBeginOverlap(BC_Battery)
  (params (OverlappedComponent :type Primitive%20Component%20Object%20Reference) (OtherActor :type Actor%20Object%20Reference) (OtherComp :type Primitive%20Component%20Object%20Reference) (OtherBodyIndex :type Integer) (bFromSweep :type Boolean) (SweepResult :type Hit%20Result%20Structure%20%28by%20ref%29))
  (bind _asbp_electronics (Utilities|Casting|CastToBP_Electronics OtherActor))
  (if (== (Variables|/Game/MyLogic/BP_Electronics.BP_Electronics_C|GetCompNumber _asbp_electronics) 3)
    (Utilities|FlowControl|DoOnce false
      (:Completed
        (Actor|DestroyActor _asbp_electronics)
        (Rendering|SetVisibility (Variables|Default|GetSM_Battery) true false)))
    (else
      (bind _output_get (Variables|Default|SetErrorCount (+ (Variables|Default|GetErrorCount) 1)))
      (Development|PrintString (Utilities|String|Append "Текущее количество ошибок" (Utilities|String|ToString(Integer) _output_get) ". Нееверная установка компонента"))
      (CallFunction|ErrorCounter _output_get))))

(fn ConstructionScript)

(fn ErrorCounter
  (params (Errors :type Integer))
  (return 0))