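; 3D printer actor that spawns printed parts in the world when its PrintButtonPressed event fires.
; The event loops over the requested amount, spawning base, wheels and mounts by loop index, spaced along world X from the root plus an offset.
; The passed part index is stored but unused.
; The invalid-count error never prints because its range check requires both above two and at most zero.
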(event EventPrintButtonPressed
  (params (CurrentPartIndex :type Integer) (PartAmount :type Integer) (InfillPercent :type Integer) (SupportsEnable :type Boolean))
  (bind _defaultsceneroot (Variables|Default|GetDefaultSceneRoot))
  (bind _returnvalue (Transformation|GetWorldLocation _defaultsceneroot))
  (Variables|Default|SetCurrentPartIndex CurrentPartIndex)
  (bind _output_get (Variables|Default|SetNumberOfPrints PartAmount))
  (if (and (> _output_get 2) (<= _output_get 0))
    (Development|PrintString "Выьрано непарвильное количество деталей")
    (else
      (for _index (range 0 (- (Variables|Default|GetNumberOfPrints) 1))
        (if (== _index 0)
          (Game|SpawnActorfromClass "/Game/MyLogic/BP_PrintedBase.BP_PrintedBase_C" (Math|Transform|MakeTransform (Math|Vector|MakeVector (+ (* _index (Variables|Default|GetPacing)) (.x _returnvalue) (Variables|Default|GetOffset)) (.y _returnvalue) (.z _returnvalue)) "0, 0, 0" "1,1,1") "Undefined" 0 0)
          (elif (== _index 1)
            (Game|SpawnActorfromClass "/Game/MyLogic/BP_PrintedWheels.BP_PrintedWheels_C" (Math|Transform|MakeTransform (Math|Vector|MakeVector (+ (* _index (Variables|Default|GetPacing)) (.x _returnvalue) (Variables|Default|GetOffset)) (.y _returnvalue) (.z _returnvalue)) "0, 0, 0" "1,1,1") "Undefined" 0 0)
            (elif (== _index 2)
              (Game|SpawnActorfromClass "/Game/MyLogic/BP_PrintedMounts.BP_PrintedMounts_C" (Math|Transform|MakeTransform (Math|Vector|MakeVector (+ (* _index (Variables|Default|GetPacing)) (.x _returnvalue) (Variables|Default|GetOffset)) (.y _returnvalue) (.z _returnvalue)) "0, 0, 0" "1,1,1") "Undefined" 0 0))))))))

(fn ConstructionScript)